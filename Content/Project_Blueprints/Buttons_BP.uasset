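; Three-button puzzle Blueprint that opens a linked door once all three buttons are pressed.
; Each button's trigger box sets a proximity flag and prints an 'E' prompt for any overlapping actor.
; Pressing E nearby latches that button once and lowers its pillar through MoveComponentTo on timeline updates.
; Those same updates check all three pressed flags and call MoveDoor on DoorBP, potentially repeatedly.
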(event OnComponentBeginOverlap(ButtonBox3)
  (params (OverlappedComponent :type Primitive%20Component%20Object%20Reference) (OtherActor :type Actor%20Object%20Reference) (OtherComp :type Primitive%20Component%20Object%20Reference) (OtherBodyIndex :type Integer) (bFromSweep :type Boolean) (SweepResult :type Hit%20Result%20Structure%20%28by%20ref%29))
  ;[1 1 1] Near Button 3?
  (Utilities|FlowControl|DoOnce false
    (:Completed
      (Variables|Default|SetNearButton3 true)
      (Development|PrintString "Press 'E' to interact"))))

(event OnComponentEndOverlap(ButtonBox3)
  (params (OverlappedComponent :type Primitive%20Component%20Object%20Reference) (OtherActor :type Actor%20Object%20Reference) (OtherComp :type Primitive%20Component%20Object%20Reference) (OtherBodyIndex :type Integer))
  ;[1 1 1] Near Button 3?
  (Variables|Default|SetNearButton3 false)
  (Utilities|FlowControl|DoOnce false) ; enters at Reset
)

(event OnComponentBeginOverlap(ButtonBox1)
  (params (OverlappedComponent :type Primitive%20Component%20Object%20Reference) (OtherActor :type Actor%20Object%20Reference) (OtherComp :type Primitive%20Component%20Object%20Reference) (OtherBodyIndex :type Integer) (bFromSweep :type Boolean) (SweepResult :type Hit%20Result%20Structure%20%28by%20ref%29))
  ;[1 1 1] Near Button 1?
  (Utilities|FlowControl|DoOnce false
    (:Completed
      (Variables|Default|SetNearButton1 true)
      (Development|PrintString "Press 'E' to interact"))))

(event OnComponentEndOverlap(ButtonBox1)
  (params (OverlappedComponent :type Primitive%20Component%20Object%20Reference) (OtherActor :type Actor%20Object%20Reference) (OtherComp :type Primitive%20Component%20Object%20Reference) (OtherBodyIndex :type Integer))
  ;[1 1 1] Near Button 1?
  (Variables|Default|SetNearButton1 false)
  (Utilities|FlowControl|DoOnce false) ; enters at Reset
)

(event OnComponentBeginOverlap(ButtonBox2)
  (params (OverlappedComponent :type Primitive%20Component%20Object%20Reference) (OtherActor :type Actor%20Object%20Reference) (OtherComp :type Primitive%20Component%20Object%20Reference) (OtherBodyIndex :type Integer) (bFromSweep :type Boolean) (SweepResult :type Hit%20Result%20Structure%20%28by%20ref%29))
  ;[1 1 1] Near Button 2?
  (Utilities|FlowControl|DoOnce false
    (:Completed
      (Variables|Default|SetNearButton2 true)
      (Development|PrintString "Press 'E' to interact"))))

(event OnComponentEndOverlap(ButtonBox2)
  (params (OverlappedComponent :type Primitive%20Component%20Object%20Reference) (OtherActor :type Actor%20Object%20Reference) (OtherComp :type Primitive%20Component%20Object%20Reference) (OtherBodyIndex :type Integer))
  ;[1 1 1] Near Button 2?
  (Variables|Default|SetNearButton2 false)
  (Utilities|FlowControl|DoOnce false) ; enters at Reset
)

(event EventBeginPlay
  ;[1 1 1] Enable Input
  (Input|EnableInput (Game|GetPlayerCharacter 0) (Game|GetPlayerController 0)))

(event Input|KeyboardEvents|E
  (params (Key :type Key%20Structure :default "None"))
  ;[1 1 1] Press Buttons
  (:Pressed
    (Utilities|FlowControl|Sequence
      (:then_0
        (if (Variables|Default|GetNearButton1)
          (Utilities|FlowControl|DoOnce false
            (:Completed
              (Variables|Default|SetButton1Pressed true)
              (bind _animationtime (Timeline|PillarLowers Play)
                (:Update
                  (Components|MoveComponentTo (Variables|Default|GetPillar1) (- (Variables|/Script/Engine.SceneComponent|GetRelativeLocation (Variables|Default|GetPillar1)) "0, 0,2.000000") "0, 0, 0" false false _animationtime false)
                  (if (Math|Boolean|ANDBoolean (Variables|Default|GetButton1Pressed) (Variables|Default|GetButton2Pressed) (Variables|Default|GetButton3Pressed)) :!label _label
                    (Default|MoveDoor (Variables|Default|GetDoor_BP)))))))))
      (:then_1
        (if (Variables|Default|GetNearButton2)
          (Utilities|FlowControl|DoOnce false
            (:Completed
              (Variables|Default|SetButton2Pressed true)
              (bind _animationtime_2 (Timeline|Timeline_0 Play)
                (:Update
                  (Components|MoveComponentTo (Variables|Default|GetPillar2) (- (Variables|/Script/Engine.SceneComponent|GetRelativeLocation (Variables|Default|GetPillar2)) "0, 0,2.000000") "0, 0, 0" false false _animationtime_2 false)
                  (goto _label)))))))
      (:then_2
        (if (Variables|Default|GetNearButton3)
          (Utilities|FlowControl|DoOnce false
            (:Completed
              (Variables|Default|SetButton3Pressed true)
              (bind _animationtime_3 (Timeline|Timeline_1 Play)
                (:Update
                  (Components|MoveComponentTo (Variables|Default|GetPillar3) (- (Variables|/Script/Engine.SceneComponent|GetRelativeLocation (Variables|Default|GetPillar3)) "0, 0,2.000000") "0, 0, 0" false false _animationtime_3 false)
                  (goto _label))))))))))

(fn ConstructionScript)