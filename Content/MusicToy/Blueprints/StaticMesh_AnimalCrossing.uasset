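; Breakable music toy, themed on Animal Crossing by its name, that plays the "8 AM" track when its destructible mesh fractures.
; The construction script assigns BaseMesh to the Destructible component.
; On fracture it spawns the attenuated sound at a stored location, starting partway into the track with auto-destroy off.
; After a delay it restores the component's relative location and reapplies BaseMesh to reset the broken object.
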(event OnComponentFracture(Destructible)
  (Audio|SpawnSoundatLocation "/Game/MusicToy/Boden_Toy01/sounds/tracks/021_-_8_AM.021_-_8_AM" (Variables|Default|GetLocation) "0, 0, 0" 1.0 1.0 6.0 "/Game/MusicToy/Boden_Toy01/sounds/Dragonborn.Dragonborn" 0 false)
  (Utilities|FlowControl|Delay 1e+01)
  (Transformation|SetRelativeLocation (Variables|Default|GetDestructible) (Variables|Default|Getoriginal%20location) false false)
  (CallFunction|SetDestructibleMesh (Variables|Default|GetDestructible) (.Base%20mesh (Variables|Default|GetBase%20mesh))))

(fn ConstructionScript
  (Variables|Default|SetDestructibleMesh (Variables|Default|GetDestructible) (.Base%20mesh (Variables|Default|GetBase%20mesh))))