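; Destructible music toy actor that plays a 2D sound when broken and then restores itself.
; The construction script assigns BaseMesh to the Destructible component.
; On component fracture it plays the sound, waits briefly, then moves the component back to OriginalLocation and reapplies BaseMesh to reset it.
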(event OnComponentFracture(Destructible)
  (params (HitPoint :type Vector%20%28by%20ref%29 :default "0, 0, 0") (HitDirection :type Vector%20%28by%20ref%29 :default "0, 0, 0"))
  (Audio|PlaySound2D 0 1.0 1.0 0.0 0 0)
  (Utilities|FlowControl|Delay 2.0)
  (Transformation|SetRelativeLocation (Variables|Default|GetDestructible) (Variables|Default|Getoriginal%20location) false false)
  (Class|DestructibleComponent|SetDestructibleMesh (Variables|Default|GetDestructible) (Variables|Default|GetBase%20mesh)))

(fn ConstructionScript
  (Variables|/Script/ApexDestruction.DestructibleComponent|SetDestructibleMesh (Variables|Default|GetDestructible) (Variables|Default|GetBase%20mesh)))